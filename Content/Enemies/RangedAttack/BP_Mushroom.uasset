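; Ranged mushroom enemy that faces the player along the X axis and attacks on a looping timer once the player enters its box.
; Attacks jump to a PaperZD animation node, while a separate SpawnProjectile event fires the projectile from SpawnPoint.
; Damage updates the health bar widget, then either knocks it back with a hurt animation or plays death and destroys it after a delay.
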(event OnComponentBeginOverlap(Box)
  (params (OverlappedComponent :type Primitive%20Component%20Object%20Reference) (OtherActor :type Actor%20Object%20Reference) (OtherComp :type Primitive%20Component%20Object%20Reference) (OtherBodyIndex :type Integer) (bFromSweep :type Boolean) (SweepResult :type Hit%20Result%20Structure%20%28by%20ref%29))
  (if (== OtherActor (Game|GetPlayerCharacter 0))
    (Utilities|Time|SetTimerbyEvent (delegate Custom|Mushroom%20Attack) 1.0 true)))

(event Custom|Handle%20Rotation
  (if (not (Variables|DoNotEdit|GetisDead?))
    (if (< (.x (Math|Vector|GetUnitDirection(Vector) (Transformation|GetActorLocation (Game|GetPlayerCharacter 0)) (Transformation|GetActorLocation))) 0.0)
      (Transformation|SetActorRotation "0, 0, 0")
      (else
        (Transformation|SetActorRotation "0,180.000000, 0")))))

(event Custom|Mushroom%20Attack
  (if (not (or (Variables|DoNotEdit|GetisDead?) (AI|Components|NavMovement|IsFalling (Variables|Character|GetCharacterMovement))))
    (Class|PaperZDAnimInstance|JumptoNode (Variables|/Script/PaperZD.PaperZDAnimationComponent|GetAnimInstance (Variables|Default|GetAnimationComponent)) (Variables|Default|GetattackJumpNode) "None")))

(event Custom|Spawn%20Projectile
  (Game|SpawnActorfromClass (Variables|Default|GetProjectileClass) (Math|Transform|MakeTransform (Transformation|GetWorldLocation (Variables|Default|GetspawnPoint)) (Transformation|GetActorRotation) "1.000000,1.000000,1.000000") "Undefined" 0 0))

(event EventBeginPlay
  (Variables|Default|SetmaxHealth (Variables|Default|Gethealth))
  (bind _aswb_ranged_health_bar (Utilities|Casting|CastToWB_RangedHealthBar (UserInterface|GetWidget (Variables|Default|GetWidget))))
  (bind _output_get (Variables|DoNotEdit|SetAs%20WB%20Ranged%20Health%20Bar _aswb_ranged_health_bar))
  (Variables|/Game/Widgets/WB_RangedHealthBar.WB_RangedHealthBar_C|SetmushroomRef _output_get self))

(event Game|Damage|EventAnyDamage
  (params (Damage :type Float%20%28single-precision%29) (DamageType :type Damage%20Type%20Object%20Reference) (InstigatedBy :type Controller%20Object%20Reference) (DamageCauser :type Actor%20Object%20Reference))
  ;[1 1 1] Handle Damage
  (Variables|Default|Sethealth (- (Variables|Default|Gethealth) Damage))
  (Default|UpdateHealthBar (Variables|DoNotEdit|GetAs%20WB%20Ranged%20Health%20Bar))
  (Variables|DoNotEdit|SetenemyDamaged? true)
  (if (<= (Variables|Default|Gethealth) 0.0)
    (Class|PaperZDAnimInstance|JumptoNode (Variables|/Script/PaperZD.PaperZDAnimationComponent|GetAnimInstance (Variables|Default|GetAnimationComponent)) (Variables|Default|GetdeathJumpNode) "None")
    (Variables|DoNotEdit|SetisDead? true)
    (Rendering|SetVisibility (Variables|Default|GetWidget) false false)
    (Collision|SetCollisionProfileName (Variables|Default|GetCapsuleComponent) "OverlapOnlyPawn" true :!class /Script/Engine.PrimitiveComponent)
    (Utilities|FlowControl|Delay 3.0)
    (Actor|DestroyActor)
    (else
      (Character|LaunchCharacter (Math|Vector|MakeVector (* (select (< (.x (Math|Vector|GetUnitDirection(Vector) (Transformation|GetActorLocation DamageCauser) (Transformation|GetActorLocation))) 0.0) 1.0 -1.0) -8e+02) 0.0 1e+02) true true)
      (Class|PaperZDAnimInstance|JumptoNode (Variables|/Script/PaperZD.PaperZDAnimationComponent|GetAnimInstance (Variables|Default|GetAnimationComponent)) (Variables|Default|GetdamagedJumpNode) "None")
      (Rendering|SetVisibility (Variables|Default|GetWidget) true false)
      (Utilities|FlowControl|RetriggerableDelay 0.1)
      (Variables|DoNotEdit|SetenemyDamaged? false))))

(event EventTick
  (params (DeltaSeconds :type Float%20%28single-precision%29))
  (CallFunction|HandleRotation))

(fn ConstructionScript)