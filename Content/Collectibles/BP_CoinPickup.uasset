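; Coin pickup actor that adds to the player's coin count and converts the hundredth coin into an extra life.
; A sphere overlap casts the other actor to BP_Player and changes its Coins and Lives directly, then destroys the pickup.
; At 99 coins it resets Coins to zero, adds a life and refreshes only the HUD's lives; otherwise it increments Coins and refreshes the coin display.
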(event OnComponentBeginOverlap(Sphere)
  (params (OverlappedComponent :type Primitive%20Component%20Object%20Reference) (OtherActor :type Actor%20Object%20Reference) (OtherComp :type Primitive%20Component%20Object%20Reference) (OtherBodyIndex :type Integer) (bFromSweep :type Boolean) (SweepResult :type Hit%20Result%20Structure%20%28by%20ref%29))
  (bind _asbp_player (Utilities|Casting|CastToBP_Player OtherActor))
  (Variables|Default|SetAs%20BP%20Player _asbp_player)
  (if (== (Variables|/Game/PlayerCharacter/BP_Player.BP_Player_C|Getcoins _asbp_player) 99.0)
    (Variables|/Game/PlayerCharacter/BP_Player.BP_Player_C|Setcoins (Variables|Default|GetAs%20BP%20Player) 0.0)
    (Variables|/Game/PlayerCharacter/BP_Player.BP_Player_C|Setlives (Variables|Default|GetAs%20BP%20Player) (+ (Variables|/Game/PlayerCharacter/BP_Player.BP_Player_C|Getlives (Variables|Default|GetAs%20BP%20Player)) 1.0))
    (Default|UpdateLives (Variables|/Game/PlayerCharacter/BP_Player.BP_Player_C|GethudRef (Variables|Default|GetAs%20BP%20Player)))
    (Actor|DestroyActor)
    (else
      (Variables|/Game/PlayerCharacter/BP_Player.BP_Player_C|Setcoins (Variables|Default|GetAs%20BP%20Player) (+ (Variables|/Game/PlayerCharacter/BP_Player.BP_Player_C|Getcoins (Variables|Default|GetAs%20BP%20Player)) 1.0))
      (Default|UpdateCoins (Variables|/Game/PlayerCharacter/BP_Player.BP_Player_C|GethudRef (Variables|Default|GetAs%20BP%20Player)))
      (Actor|DestroyActor))))

(event EventBeginPlay)

(event Collision|EventActorBeginOverlap
  (params (OtherActor :type Actor%20Object%20Reference)))

(event EventTick
  (params (DeltaSeconds :type Float%20%28single-precision%29)))

(fn ConstructionScript)