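; BP_ProjectilePickup is a collectible that refills the player's projectile count.
; When BP_Player overlaps its sphere below maximum capacity, it adds a fixed amount, clamped to that maximum.
; It then refreshes the count through the player's HUD reference and destroys itself.
; A player already at maximum leaves the pickup in the world.
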(event OnComponentBeginOverlap(Sphere)
  (params (OverlappedComponent :type Primitive%20Component%20Object%20Reference) (OtherActor :type Actor%20Object%20Reference) (OtherComp :type Primitive%20Component%20Object%20Reference) (OtherBodyIndex :type Integer) (bFromSweep :type Boolean) (SweepResult :type Hit%20Result%20Structure%20%28by%20ref%29))
  (bind _asbp_player (Utilities|Casting|CastToBP_Player OtherActor))
  (bind _output_get (Variables|Default|SetAs%20BP%20Player _asbp_player))
  (if (not (== (Variables|/Game/PlayerCharacter/BP_Player.BP_Player_C|Getprojectile _output_get) (Variables|/Game/PlayerCharacter/BP_Player.BP_Player_C|GetmaxProjectile _output_get)))
    (Variables|/Game/PlayerCharacter/BP_Player.BP_Player_C|Setprojectile (Variables|Default|GetAs%20BP%20Player) (Math|Integer|Clamp(Integer) (+ (Variables|/Game/PlayerCharacter/BP_Player.BP_Player_C|Getprojectile (Variables|Default|GetAs%20BP%20Player)) 5) 1 (Variables|/Game/PlayerCharacter/BP_Player.BP_Player_C|GetmaxProjectile (Variables|Default|GetAs%20BP%20Player))))
    (Default|UpdateProjectile (Variables|/Game/PlayerCharacter/BP_Player.BP_Player_C|GethudRef (Variables|Default|GetAs%20BP%20Player)))
    (Actor|DestroyActor)))

(event EventBeginPlay)

(event Collision|EventActorBeginOverlap
  (params (OtherActor :type Actor%20Object%20Reference)))

(event EventTick
  (params (DeltaSeconds :type Float%20%28single-precision%29)))

(fn ConstructionScript)