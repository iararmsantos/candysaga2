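; Health pickup actor that restores a player's health when they touch its sphere.
; On sphere overlap it casts to BP_Player and does nothing if health already equals the maximum, leaving the pickup in place.
; Otherwise it adds HealthToGive, clamped between one and max health, passes the truncated heal amount to the HUD's ShowHearts, and destroys itself.
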(event OnComponentBeginOverlap(Sphere)
  (params (OverlappedComponent :type Primitive%20Component%20Object%20Reference) (OtherActor :type Actor%20Object%20Reference) (OtherComp :type Primitive%20Component%20Object%20Reference) (OtherBodyIndex :type Integer) (bFromSweep :type Boolean) (SweepResult :type Hit%20Result%20Structure%20%28by%20ref%29))
  (bind _asbp_player (Utilities|Casting|CastToBP_Player OtherActor))
  (bind _output_get (Variables|Default|SetAs%20BP%20Player _asbp_player))
  (if (not (== (Variables|/Game/PlayerCharacter/BP_Player.BP_Player_C|Gethealth _output_get) (Variables|/Game/PlayerCharacter/BP_Player.BP_Player_C|GetmaxHealth _output_get)))
    (Variables|/Game/PlayerCharacter/BP_Player.BP_Player_C|Sethealth (Variables|Default|GetAs%20BP%20Player) (Math|Float|Clamp(Float) (+ (Variables|/Game/PlayerCharacter/BP_Player.BP_Player_C|Gethealth (Variables|Default|GetAs%20BP%20Player)) (Variables|Default|GethealthToGive)) 1.0 (Variables|/Game/PlayerCharacter/BP_Player.BP_Player_C|GetmaxHealth (Variables|Default|GetAs%20BP%20Player))))
    (Default|ShowHearts (Variables|/Game/PlayerCharacter/BP_Player.BP_Player_C|GethudRef (Variables|Default|GetAs%20BP%20Player)) (Math|Float|Truncate (Variables|Default|GethealthToGive)))
    (Actor|DestroyActor)))

(event EventBeginPlay)

(event Collision|EventActorBeginOverlap
  (params (OtherActor :type Actor%20Object%20Reference)))

(event EventTick
  (params (DeltaSeconds :type Float%20%28single-precision%29)))

(fn ConstructionScript)